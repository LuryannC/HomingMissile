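; Bee projectile Blueprint that applies its action, scaled by a base value, to actors its sphere overlaps, ignoring its owner.
; CanTarget accepts any target whose projectile team message is not Pollen.
; OnEndPurpose prints a debug message and sets PendingToKill once, while the SetLifeSpan call is left disconnected.
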(event OnComponentBeginOverlap(SphereComponent)
  (params (OverlappedComponent :type Primitive%20Component%20Object%20Reference) (OtherActor :type Actor%20Object%20Reference) (OtherComp :type Primitive%20Component%20Object%20Reference) (OtherBodyIndex :type Integer) (bFromSweep :type Boolean) (SweepResult :type Hit%20Result%20Structure%20%28by%20ref%29))
  (if (not (== OtherActor (Components|GetOwner)))
    (Class|HomingProjectileBase|PerformAction OtherActor (Variables|Default|GetActionBaseValue))))

(event EventBeginPlay)

(event Collision|EventActorBeginOverlap
  (params (OtherActor :type Actor%20Object%20Reference)))

(event EventTick
  (params (DeltaSeconds :type Float%20%28single-precision%29)))

(event EventOnEndPurpose
  (if (not (Variables|Default|GetbPendingToKill))
    (Development|PrintString (Utilities|String|Append (Utilities|GetDisplayName self) " Has no purpose anymore"))
    (Variables|Default|SetbPendingToKill true)))

(fn ConstructionScript)

(fn CanTarget
  (params (InTarget :type Actor%20Object%20Reference))
  (bind _returnvalue (Class|HomingProjectileTargetInterface|GetProjectileTeam(Message) InTarget))
  (return (!= _returnvalue (Math|Byte|MakeLiteralByte (Utilities|Enum|LiteralenumEEntityTeam "Pollen")))))