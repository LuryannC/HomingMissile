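; Projectile actor for worker bees in the Bee example, belonging to the Bee team and targeting actors of the Pollen team.
; On sphere overlap with any actor other than its owner, it calls PerformAction on that actor with a random integer amount.
; Targeting functions define the team rules: CanTarget compares the target's projectile team to Pollen, and CanBeTargeted always returns true.
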(event OnComponentBeginOverlap(SphereComponent)
  (params (OverlappedComponent :type Primitive%20Component%20Object%20Reference) (OtherActor :type Actor%20Object%20Reference) (OtherComp :type Primitive%20Component%20Object%20Reference) (OtherBodyIndex :type Integer) (bFromSweep :type Boolean) (SweepResult :type Hit%20Result%20Structure%20%28by%20ref%29))
  (if (not (== OtherActor (Components|GetOwner)))
    (Class|HomingProjectileBase|PerformAction OtherActor (Math|Random|RandomIntegerinRange 1 100))))

(event EventBeginPlay)

(event Collision|EventActorBeginOverlap
  (params (OtherActor :type Actor%20Object%20Reference)))

(event EventTick
  (params (DeltaSeconds :type Float%20%28single-precision%29)))

(fn ConstructionScript)

(fn CanTarget
  (params (InTarget :type Actor%20Object%20Reference))
  (bind _returnvalue (Class|HomingProjectileTargetInterface|GetProjectileTeam(Message) InTarget))
  (return (== _returnvalue (Math|Byte|MakeLiteralByte (Utilities|Enum|LiteralenumEEntityTeam "Pollen")))))

(fn CanbeTargeted
  (return true))

(fn GetProjectileTeam
  (return (Utilities|Enum|LiteralenumEEntityTeam "Bee")))